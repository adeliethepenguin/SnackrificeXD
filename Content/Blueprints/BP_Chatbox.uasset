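; BP_Chatbox steps through an array of dialogue lines, showing one in a textbox widget on each ShowText call.
; While talking, it stops BP_ThirdPersonCharacter12's movement and sets an idle flipbook.
; Frog and bird variants play narration sounds by line index; others restart an advance sound, and a random switch does nothing.
; After the last line it restores movement, resumes the walk flipbook if moving, removes the widget and resets.
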(event EventShowText
  (if (< (Variables|Default|GettalkIndex) (Utilities|Array|Length (Variables|Default|Gettext)))
    (bind _outactors (Actor|GetAllActorsOfClass "/Game/ThirdPerson/Blueprints/BP_ThirdPersonCharacter12.BP_ThirdPersonCharacter12_C"))
    (Variables|/Game/ThirdPerson/Blueprints/BP_ThirdPersonCharacter12.BP_ThirdPersonCharacter12_C|SetCanMove (Utilities|Array|Get(acopy) _outactors) false)
    (Sprite|SetFlipbook (Variables|/Game/ThirdPerson/Blueprints/BP_ThirdPersonCharacter12.BP_ThirdPersonCharacter12_C|GetDogby (Utilities|Array|Get(acopy) _outactors)) "/Game/Sprites/Other_Guys/lehamster/HamIdleBrighterReal1.HamIdleBrighterReal1")
    (Variables|Default|GetUI
      (:then
        _)
      (:else
        (bind _returnvalue (UserInterface|CreateWidget "/Game/Blueprints/UB_TextboxUI.UB_TextboxUI_C" (Game|GetPlayerController 0)))
        (bind _output_get (Variables|Default|SetUI _returnvalue))
        (UserInterface|Viewport|AddtoViewport _output_get 0)))
    (Rendering|Components|TextRender|SetText (Variables|/Game/Blueprints/UB_TextboxUI.UB_TextboxUI_C|GetTalker (Variables|Default|GetUI)) (Utilities|Text|ToText(String) (Utilities|Array|Get(acopy) (Variables|Default|Gettext) (Variables|Default|GettalkIndex))))
    (Math|Integer|IncrementInt (Variables|Default|GettalkIndex)
      (:%20%20
        (switch int (Math|Random|RandomIntegerinRange 0 2)
          (:Default
            _)
          (:0
            _)
          (:1
            _)
          (:2
            _))
        (if (Variables|Default|GetIsFrog)
          (switch int (- (Variables|Default|GettalkIndex) 1)
            (:0
              (Audio|SpawnSound2D "/Game/Sounds/soundasignemtn/narration0.narration0" 1.0 1.0 0.0 0))
            (:1
              (Audio|SpawnSound2D "/Game/Sounds/soundasignemtn/narrationfrog.narrationfrog" 1.0 1.0 0.0 0))
            (:2
              (Audio|SpawnSound2D "/Game/Sounds/soundasignemtn/narration1.narration1" 1.0 1.0 0.0 0)))
          (elif (Variables|Default|GetIsBird)
            (switch int (- (Variables|Default|GettalkIndex) 1)
              (:0
                (Audio|SpawnSound2D "/Game/Sounds/soundasignemtn/narration0.narration0" 1.0 1.0 0.0 0))
              (:1
                (Audio|SpawnSound2D "/Game/Sounds/soundasignemtn/narrationbird.narrationbird" 1.0 1.0 0.0 0))
              (:2
                (Audio|SpawnSound2D "/Game/Sounds/soundasignemtn/narration1.narration1" 1.0 1.0 0.0 0)))
            (else
              (if (== (Variables|Default|GetDialogueAdvanceSound) 0)
                _
                (else
                  (Audio|Components|Audio|Stop (Variables|Default|GetDialogueAdvanceSound))))
              (bind _returnvalue_2 (Audio|SpawnSound2D "/Game/Sounds/dialogueadvancements.dialogueadvancements" 1.0 1.0 0.0 0))
              (Variables|Default|SetDialogueAdvanceSound _returnvalue_2))))))
    (else
      (bind _outactors_2 (Actor|GetAllActorsOfClass "/Game/ThirdPerson/Blueprints/BP_ThirdPersonCharacter12.BP_ThirdPersonCharacter12_C"))
      (Variables|/Game/ThirdPerson/Blueprints/BP_ThirdPersonCharacter12.BP_ThirdPersonCharacter12_C|SetCanMove (Utilities|Array|Get(acopy) _outactors_2) true)
      (if (Variables|/Game/ThirdPerson/Blueprints/BP_ThirdPersonCharacter12.BP_ThirdPersonCharacter12_C|GetTrying2Move (Utilities|Array|Get(acopy) _outactors_2))
        (Sprite|SetFlipbook (Variables|/Game/ThirdPerson/Blueprints/BP_ThirdPersonCharacter12.BP_ThirdPersonCharacter12_C|GetDogby (Utilities|Array|Get(acopy) _outactors_2)) "/Game/Sprites/Other_Guys/lehamster/hamWalk.hamWalk"))
      (Widget|RemovefromParent (Variables|Default|GetUI))
      (Variables|Default|SettalkIndex 0)
      (Variables|Default|SetUI 0))))

(fn ConstructionScript)