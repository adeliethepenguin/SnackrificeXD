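; Boss room actor that runs a dialogue, plays a cutscene video, then loads the ActualGame level.
; ShowText, gated by Condition, freezes the player and steps through textbox lines with advance sounds, then destroys its Cube and starts the media player.
; Tick uses a Delay-driven counter or an ESCAPEEE flag to end the video, restore movement and change level.
; A separate PlayVideo event cycles sprites in a widget while boss audio plays.
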(event Custom|PlayVideo
  (bind _outactors (Actor|GetAllActorsOfClass "/Game/ThirdPerson/Blueprints/BP_ThirdPersonCharacter12.BP_ThirdPersonCharacter12_C"))
  (Variables|/Game/ThirdPerson/Blueprints/BP_ThirdPersonCharacter12.BP_ThirdPersonCharacter12_C|SetCanMove (Utilities|Array|Get(acopy) _outactors) false)
  (bind _returnvalue (UserInterface|CreateWidget "/Game/Blueprints/UB_Video.UB_Video_C"))
  (Variables|Default|SetVideo _returnvalue)
  (bind _returnvalue_2 (Audio|CreateSound2D "/Game/Sounds/beachboss.beachboss" 1.0 1.0 0.0 0))
  (bind _output_get (Variables|Default|SetAudioComponent2 _returnvalue_2))
  (Audio|Components|Audio|Play _output_get 0.0)
  (while (Audio|Components|Audio|IsPlaying (Variables|Default|GetAudioComponent2))
    (Utilities|FlowControl|Delay 1.0)
    (bind _output_get_2 (Variables|Default|SetCounter (+ (Variables|Default|GetCounter) 0.0)))
    (if (> _output_get_2 3.0)
      (Variables|Default|SetCounter 0.0)
      (Math|Integer|IncrementInt (Variables|Default|Getindex)
        (:%20%20
          (if (> (Variables|Default|Getindex) (Utilities|Array|Length (Variables|Default|GetSpritesyea)))
            (Variables|Default|Setindex 0))
          (Default|SetVideoDisplay (Variables|Default|GetVideo) (Utilities|Array|Get(acopy) (Variables|Default|GetSpritesyea) (Variables|Default|Getindex)))))))
  (Widget|RemovefromParent (Variables|Default|GetVideo))
  (bind _outactors_2 (Actor|GetAllActorsOfClass "/Game/ThirdPerson/Blueprints/BP_ThirdPersonCharacter12.BP_ThirdPersonCharacter12_C"))
  (Variables|/Game/ThirdPerson/Blueprints/BP_ThirdPersonCharacter12.BP_ThirdPersonCharacter12_C|SetCanMove (Utilities|Array|Get(acopy) _outactors_2) true))

(event EventShowText
  (Development|PrintString "a")
  (if (Variables|Default|GetCondition)
    (Development|PrintString "b")
    (if (< (Variables|Default|GetTalk%20Index) (Utilities|Array|Length (Variables|Default|Gettext)))
      (bind _outactors (Actor|GetAllActorsOfClass "/Game/ThirdPerson/Blueprints/BP_ThirdPersonCharacter12.BP_ThirdPersonCharacter12_C"))
      (Variables|/Game/ThirdPerson/Blueprints/BP_ThirdPersonCharacter12.BP_ThirdPersonCharacter12_C|SetCanMove (Utilities|Array|Get(acopy) _outactors) false)
      (Sprite|SetFlipbook (Variables|/Game/ThirdPerson/Blueprints/BP_ThirdPersonCharacter12.BP_ThirdPersonCharacter12_C|GetDogby (Utilities|Array|Get(acopy) _outactors)) "/Game/Sprites/dogby/DogbyIdle.DogbyIdle")
      (Variables|Default|GetUI
        (:then
          _)
        (:else
          (bind _returnvalue (UserInterface|CreateWidget "/Game/Blueprints/UB_TextboxUI.UB_TextboxUI_C" (Game|GetPlayerController 0)))
          (bind _output_get (Variables|Default|SetUI _returnvalue))
          (UserInterface|Viewport|AddtoViewport _output_get 0)))
      (Rendering|Components|TextRender|SetText (Variables|/Game/Blueprints/UB_TextboxUI.UB_TextboxUI_C|GetTalker (Variables|Default|GetUI)) (Utilities|Text|ToText(String) (Utilities|Array|Get(acopy) (Variables|Default|Gettext) (Variables|Default|GetTalk%20Index))))
      (Math|Integer|IncrementInt (Variables|Default|GetTalk%20Index)
        (:%20%20
          (switch int (Math|Random|RandomIntegerinRange 0 2)
            (:Default
              _)
            (:0
              _)
            (:1
              _)
            (:2
              _))
          (if (== (Variables|Default|GetDialogue%20Advance%20Sound) 0)
            _
            (else
              (Audio|Components|Audio|Stop (Variables|Default|GetDialogue%20Advance%20Sound))))
          (bind _returnvalue_2 (Audio|SpawnSound2D "/Game/Sounds/dialogueadvancements.dialogueadvancements" 1.0 1.0 0.0 0))
          (Variables|Default|SetDialogue%20Advance%20Sound _returnvalue_2)))
      (else
        (bind _outactors_2 (Actor|GetAllActorsOfClass "/Game/ThirdPerson/Blueprints/BP_ThirdPersonCharacter12.BP_ThirdPersonCharacter12_C"))
        (Variables|/Game/ThirdPerson/Blueprints/BP_ThirdPersonCharacter12.BP_ThirdPersonCharacter12_C|SetCanMove (Utilities|Array|Get(acopy) _outactors_2) false)
        (if (Variables|/Game/ThirdPerson/Blueprints/BP_ThirdPersonCharacter12.BP_ThirdPersonCharacter12_C|GetTrying2Move (Utilities|Array|Get(acopy) _outactors_2))
          (Sprite|SetFlipbook (Variables|/Game/ThirdPerson/Blueprints/BP_ThirdPersonCharacter12.BP_ThirdPersonCharacter12_C|GetDogby (Utilities|Array|Get(acopy) _outactors_2)) "/Game/Sprites/dogby/Walk/FB_DogbyWalk.FB_DogbyWalk"))
        (Widget|RemovefromParent (Variables|Default|GetUI))
        (Variables|Default|SetTalk%20Index 0)
        (Variables|Default|SetUI 0)
        (Development|PrintString "Bro")
        (Variables|Default|SetCondition false)
        (Media|MediaPlayer|OpenSource (Variables|Default|GetNewVar) "/Game/Movies/1444.1444")
        (Media|MediaPlayer|Play (Variables|Default|GetNewVar) :!class /Script/MediaAssets.MediaPlayer)
        (bind _outactors_3 (Actor|GetAllActorsOfClass "/Game/ThirdPerson/Blueprints/BP_ThirdPersonCharacter12.BP_ThirdPersonCharacter12_C"))
        (Variables|/Game/ThirdPerson/Blueprints/BP_ThirdPersonCharacter12.BP_ThirdPersonCharacter12_C|SetCanMove (Utilities|Array|Get(acopy) _outactors_3) false)
        (Variables|Default|Set2 true)
        (Components|DestroyComponent (Variables|Default|GetCube))
        (Variables|Default|SetNewVar_0 true)))
    (else
      (Development|PrintString "cc"))))

(event EventTick
  (params (DeltaSeconds :type Float%20%28single-precision%29))
  (if (Variables|Default|GetNewVar_0)
    (if (or (> (Variables|Default|GetNewCounter3) 42.0) (Variables|Default|GetESCAPEEE))
      (Variables|Default|SetNewVar_0 false)
      (bind _outactors (Actor|GetAllActorsOfClass "/Game/ThirdPerson/Blueprints/BP_ThirdPersonCharacter12.BP_ThirdPersonCharacter12_C"))
      (Variables|/Game/ThirdPerson/Blueprints/BP_ThirdPersonCharacter12.BP_ThirdPersonCharacter12_C|SetCanMove (Utilities|Array|Get(acopy) _outactors) true)
      (Media|MediaPlayer|Close (Variables|Default|GetNewVar) :!class /Script/MediaAssets.MediaPlayer)
      (Game|OpenLevel(byName) "ActualGame")
      (else
        (Utilities|FlowControl|Delay 1.0)
        (Variables|Default|SetNewCounter3 (+ (Variables|Default|GetNewCounter3) 1.0))))))

(fn ConstructionScript)