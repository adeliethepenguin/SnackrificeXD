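; Elevator actor that plays a dialogue, opens, then carries the player on to the BossRoom level.
; Each ShowText call on the closed sprite advances a textbox widget with a sound while freezing the Dogby character's movement.
; After the last line it restores movement, swaps to the open sprite, disables collision and pings.
; An end overlap past a Y threshold closes it, plays a sound and loads BossRoom after a delay.
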(event EventShowText
  (Development|PrintString "a")
  (if (== (Sprite|GetSprite (Variables|Default|GetPaperSprite)) "/Game/Sprites/Misc/elevator_Sprite.elevator_Sprite")
    (Development|PrintString "b")
    (if (< (Variables|Default|GetTalk%20Index) (Utilities|Array|Length (Variables|Default|Gettext)))
      (bind _outactors (Actor|GetAllActorsOfClass "/Game/ThirdPerson/Blueprints/BP_ThirdPersonCharacter12.BP_ThirdPersonCharacter12_C"))
      (Variables|/Game/ThirdPerson/Blueprints/BP_ThirdPersonCharacter12.BP_ThirdPersonCharacter12_C|SetCanMove (Utilities|Array|Get(acopy) _outactors) false)
      (Sprite|SetFlipbook (Variables|/Game/ThirdPerson/Blueprints/BP_ThirdPersonCharacter12.BP_ThirdPersonCharacter12_C|GetDogby (Utilities|Array|Get(acopy) _outactors)) "/Game/Sprites/dogby/DogbyIdle.DogbyIdle")
      (Variables|Default|GetUI
        (:then
          _)
        (:else
          (bind _returnvalue (UserInterface|CreateWidget "/Game/Blueprints/UB_TextboxUI.UB_TextboxUI_C" (Game|GetPlayerController 0)))
          (bind _output_get (Variables|Default|SetUI _returnvalue))
          (UserInterface|Viewport|AddtoViewport _output_get 0)))
      (Rendering|Components|TextRender|SetText (Variables|/Game/Blueprints/UB_TextboxUI.UB_TextboxUI_C|GetTalker (Variables|Default|GetUI)) (Utilities|Text|ToText(String) (Utilities|Array|Get(acopy) (Variables|Default|Gettext) (Variables|Default|GetTalk%20Index))))
      (Math|Integer|IncrementInt (Variables|Default|GetTalk%20Index)
        (:%20%20
          (switch int (Math|Random|RandomIntegerinRange 0 2)
            (:Default
              _)
            (:0
              _)
            (:1
              _)
            (:2
              _))
          (if (== (Variables|Default|GetDialogue%20Advance%20Sound) 0)
            _
            (else
              (Audio|Components|Audio|Stop (Variables|Default|GetDialogue%20Advance%20Sound))))
          (bind _returnvalue_2 (Audio|SpawnSound2D "/Game/Sounds/dialogueadvancements.dialogueadvancements" 1.0 1.0 0.0 0))
          (Variables|Default|SetDialogue%20Advance%20Sound _returnvalue_2)))
      (else
        (bind _outactors_2 (Actor|GetAllActorsOfClass "/Game/ThirdPerson/Blueprints/BP_ThirdPersonCharacter12.BP_ThirdPersonCharacter12_C"))
        (Variables|/Game/ThirdPerson/Blueprints/BP_ThirdPersonCharacter12.BP_ThirdPersonCharacter12_C|SetCanMove (Utilities|Array|Get(acopy) _outactors_2) true)
        (if (Variables|/Game/ThirdPerson/Blueprints/BP_ThirdPersonCharacter12.BP_ThirdPersonCharacter12_C|GetTrying2Move (Utilities|Array|Get(acopy) _outactors_2))
          (Sprite|SetFlipbook (Variables|/Game/ThirdPerson/Blueprints/BP_ThirdPersonCharacter12.BP_ThirdPersonCharacter12_C|GetDogby (Utilities|Array|Get(acopy) _outactors_2)) "/Game/Sprites/dogby/Walk/FB_DogbyWalk.FB_DogbyWalk"))
        (Widget|RemovefromParent (Variables|Default|GetUI))
        (Variables|Default|SetTalk%20Index 0)
        (Variables|Default|SetUI 0)
        (Rendering|Components|Sprite|SetSprite (Variables|Default|GetPaperSprite) "/Game/Sprites/Misc/elevatoropen_Sprite.elevatoropen_Sprite")
        (Collision|SetCollisionEnabled (Variables|Default|GetPaperSprite) "NoCollision")
        (Audio|SpawnSound2D "/Game/Sounds/514864__matrixxx__elevator-ping-03.514864__matrixxx__elevator-ping-03" 1.0 1.0 0.0 0)))
    (else
      (Development|PrintString "cc"))))

(event Collision|EventActorEndOverlap
  (params (OtherActor :type Actor%20Object%20Reference))
  (if (and (== (Sprite|GetSprite (Variables|Default|GetPaperSprite)) "/Game/Sprites/Misc/elevatoropen_Sprite.elevatoropen_Sprite") (< (.y (Transformation|GetActorLocation OtherActor)) 2.4e+02))
    (Variables|Default|SetNewVar false)
    (Rendering|Components|Sprite|SetSprite (Variables|Default|GetPaperSprite) "/Game/Sprites/Misc/elevator_Sprite.elevator_Sprite")
    (Collision|SetCollisionEnabled (Variables|Default|GetPaperSprite) "QueryAndPhysics")
    (Audio|SpawnSound2D "/Game/Sounds/elevatorsuccess.elevatorsuccess" 1.0 1.0 0.0 0)
    (Utilities|FlowControl|Delay 3.0)
    (Game|OpenLevel(byName) "BossRoom")))

(fn ConstructionScript)