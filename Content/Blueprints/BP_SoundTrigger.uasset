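; BP_SoundTrigger is an actor that plays a water-cooler conversation sound, getting louder as the player approaches.
; The first actor overlap, from any actor, spawns the sound quietly at the trigger's location and stores its reference, with a flag preventing replays.
; The PlayerMove event measures player distance and, inside the Sphere radius, scales volume linearly from a quiet floor, capped at full volume near the center.
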(event Custom|PlayerMove
  (bind _sphere (Variables|Default|GetSphere))
  (bind _soundref (Variables|Default|GetSoundref))
  (bind _returnvalue (Components|Sphere|GetScaledSphereRadius _sphere))
  (bind _output_get (Variables|Default|SetDistanceToPlayer (Math|Vector|VectorLength (- (Transformation|GetActorLocation) (Transformation|GetActorLocation (Game|Player|GetPlayerPawn 0))))))
  (if (<= _output_get _returnvalue)
    (if (>= (+ (/ (- _returnvalue (Variables|Default|GetDistanceToPlayer)) _returnvalue) 0.2) 1.0)
      (Audio|Components|Audio|SetVolumeMultiplier _soundref 1.0 :!class /Script/Engine.AudioComponent)
      (else
        (Audio|Components|Audio|SetVolumeMultiplier _soundref (+ (/ (- _returnvalue (Variables|Default|GetDistanceToPlayer)) _returnvalue) 0.2) :!class /Script/Engine.AudioComponent)))))

(event Collision|EventActorBeginOverlap
  (params (OtherActor :type Actor%20Object%20Reference))
  (if (not (Variables|Default|GetStartedConversation))
    (bind _returnvalue (Audio|SpawnSoundatLocation "/Game/Sounds/boringwatercoolertalk.boringwatercoolertalk" (Transformation|GetActorLocation) "0, 0, 0" 1.0 1.0 0.0 0 0))
    (Audio|Components|Audio|SetVolumeMultiplier _returnvalue 0.2 :!class /Script/Engine.AudioComponent)
    (Variables|Default|SetSoundref _returnvalue)
    (Variables|Default|SetStartedConversation true)))

(fn ConstructionScript)